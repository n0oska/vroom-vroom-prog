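; BP_Chara1 is a player-controlled, physics-driven character, viewed through a BP_Camera actor found in the level.
; BeginPlay sets a random vector material parameter (name unset), adds the IMC_Vroom input context and switches the view to that camera.
; IA_Move pushes the capsule along its forward vector while OnGround is true, and IA_Rotate yaws it.
; Tick clears OnGround every frame; nothing here sets it true.
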(event `self.ReceiveBeginPlay`
  (`MeshComponent.SetVectorParameterValueOnMaterials` (`self.Mesh`) "None" (`KismetMathLibrary.RandomUnitVector`))
  (`EnhancedInputSubsystemInterface.AddMappingContext` (pcsubsystem `EnhancedInputLocalPlayerSubsystem` (`GameplayStatics.GetPlayerController` 0)) "/Game/BP/IA_Players/IMC_Vroom.IMC_Vroom" 0 (struct))
  (bind _returnvalue (`GameplayStatics.GetActorOfClass` "/Game/BP/BP_Camera/BP_Camera.BP_Camera_C"))
  (set `self.Camera` _returnvalue)
  (`PlayerController.SetViewTargetWithBlend` (`GameplayStatics.GetPlayerController` 0) (`self.Camera`) 0.0 "VTBlend_Linear" 0.0 false))

(event `EnhancedInput|/Game/BP/IA_Players/IA_Move`
  (params (ActionValue :type "Float (double-precision)") (ElapsedSeconds :type "Float (double-precision)") (TriggeredSeconds :type "Float (double-precision)") (InputAction :type "InputAction Object Reference" :default "/Game/BP/IA_Players/IA_Move.IA_Move"))
  (:`Triggered`
    (if (`self.OnGround`)
      (`PrimitiveComponent.AddForce` (`self.CapsuleComponent`) (* (* ActionValue (`self.MoveForce`)) (`SceneComponent.GetForwardVector` (`self.CapsuleComponent`))) "None" false))))

(event `EnhancedInput|/Game/BP/IA_Players/IA_Rotate`
  (params (ActionValue :type "Float (double-precision)") (ElapsedSeconds :type "Float (double-precision)") (TriggeredSeconds :type "Float (double-precision)") (InputAction :type "InputAction Object Reference" :default "/Game/BP/IA_Players/IA_Rotate.IA_Rotate"))
  (:`Triggered`
    (`SceneComponent.K2_AddWorldRotation` (`self.CapsuleComponent`) (`KismetMathLibrary.MakeRotator` 0.0 0.0 (* ActionValue (`self.RotatioForce`))) false false)))

(event `self.ReceiveTick`
  (params (DeltaSeconds :type "Float (single-precision)"))
  (set `self.OnGround` false))

(fn `UserConstructionScript`)